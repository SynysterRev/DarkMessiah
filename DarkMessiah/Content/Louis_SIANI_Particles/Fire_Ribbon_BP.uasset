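; Fire ribbon particle actor that trails a target actor assigned through SetTarget.
; Each Tick it moves itself to the target's location without sweeping while that target is valid.
; Once the target is invalid, a one-shot guard deactivates the particle system and starts a short timer that destroys the actor, leaving time for the effect to fade.
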(event `self.ReceiveTick`
  (params (DeltaSeconds :type "Float (single-precision)"))
  (bind _target (`self.Target`))
  ;[0 1 1] Louis SIANI - Enable Ribbon and follow target
  (`/Engine/EditorBlueprintResources/StandardMacros.IsValid` _target
    (:`Is Valid`
      (`self.K2_SetActorLocation` (`self.K2_GetActorLocation` _target)))
    (:`Is Not Valid`
      (if (not (`self.TimerEnabled`))
        (set `self.TimerEnabled` true)
        (`KismetSystemLibrary.K2_SetTimer` null "Destroy" 1.0)
        (`ActorComponent.Deactivate` (`self.ParticleSystemComponent`))))))

(fn `Destroy`
  (`self.K2_DestroyActor`))

(fn `SetTarget`
  (params (target :type "Actor Object Reference"))
  (set `self.Target` target))

(fn `UserConstructionScript`)